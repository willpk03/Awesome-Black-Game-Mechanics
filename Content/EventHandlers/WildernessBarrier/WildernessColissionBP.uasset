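; WildernessColissionBP is a barrier that blocks the player until they carry the item named by its DialogueHandler.
; On any actor overlap, it asks player 0's BP_ThirdPersonCharacter whether it has that item, without checking which actor overlapped.
; If so, it disables the Cube's collision and never restores it; otherwise it runs the DialogueHandler's dialogue check and prints a debug string.
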(event `self.ReceiveActorBeginOverlap`
  (params (OtherActor :type "Actor Object Reference"))
  (bind _asbp_third_person_character (cast `/Game/ThirdPerson/Blueprints/BP_ThirdPersonCharacter` (`GameplayStatics.GetPlayerCharacter` 0)))
  (bind _hasitem (`/Game/ThirdPerson/Blueprints/BP_ThirdPersonCharacter.DoYouHaveItem` _asbp_third_person_character (`/Game/EventHandlers/WildernessBarrier/WildernessDialogueBP.neededItem` (`self.DialogueHandler`))))
  (if _hasitem
    (`PrimitiveComponent.SetCollisionEnabled` (`self.Cube`) "NoCollision")
    (else
      (`/Game/EventHandlers/WildernessBarrier/WildernessDialogueBP.fDialogueChecker` (`self.DialogueHandler`))
      (`KismetSystemLibrary.PrintString` "Hello"))))

(fn `UserConstructionScript`)