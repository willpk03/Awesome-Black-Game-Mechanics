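; Wilderness barrier dialogue handler that supplies the dialogue shown for a group of tagged barrier collision actors.
; On BeginPlay it registers itself as DialogueHandler on each matching WildernessColissionBP and sets their cube material.
; FDialogueChecker gates FHandleDiagloue, which replaces all widgets with a configured DialogueSystem and passes it to the player's GUIOpen.
; The 15-second repeat check uses frame delta instead of elapsed time, so dialogue effectively shows once.
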(event `self.ReceiveBeginPlay`
  (bind _outactors (`GameplayStatics.GetAllActorsOfClassWithTag` "/Game/EventHandlers/WildernessBarrier/WildernessColissionBP.WildernessColissionBP_C" (`self.Tag`)))
  (for _array_element _outactors
    (set `/Game/EventHandlers/WildernessBarrier/WildernessColissionBP.DialogueHandler` self _array_element)
    (`PrimitiveComponent.SetMaterial` (`/Game/EventHandlers/WildernessBarrier/WildernessColissionBP.Cube` _array_element) 0 (`self.Material`))))

(fn `fDialogueChecker`
  (bind _returnvalue (`GameplayStatics.GetWorldDeltaSeconds`))
  (bind _lastdialogue (`self.LastDialogue`))
  (if (== _lastdialogue 0.0)
    (set `self.LastDialogue` _returnvalue :!label _label)
    (`self.fHandleDiagloue`)
    (`KismetSystemLibrary.PrintString` "Hello")
    (elif (>= _returnvalue (+ _lastdialogue 15.0))
      (goto _label)
      (else
        (`KismetSystemLibrary.PrintString` "Already sent")))))

(fn `fHandleDiagloue`
  (locals (ObjectReference :type "Object Object Reference"))
  (`WidgetLayoutLibrary.RemoveAllWidgets`)
  (bind _returnvalue (`|CreateWidget` "/Game/Menu/Dialogue/dialogueSystem.dialogueSystem_C" null (`self.Name Array`) (`self.Dialogue Array`) -1 (`self.NPCImage`) (`self.Left Name`) (`self.Right Name`) (`self.Dialogue Types`) (`self.Object Reference`) (`self.Given Item`) (`self.Give Item Route`) (`self.In Str`) (`self.NPC`) (`self.Emitter`) null))
  (`UserWidget.AddToViewport` _returnvalue 0)
  (bind _asbp_third_person_character (cast `/Game/ThirdPerson/Blueprints/BP_ThirdPersonCharacter` (`GameplayStatics.GetPlayerCharacter` 0)))
  (`/Game/ThirdPerson/Blueprints/BP_ThirdPersonCharacter.GUIOpen` _asbp_third_person_character _returnvalue))

(fn `UserConstructionScript`)